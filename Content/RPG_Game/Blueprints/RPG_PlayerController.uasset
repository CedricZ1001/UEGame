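; Player controller for an RPG that drives the Shinbi character with both click-to-move and axis-based movement.
; Left click spawns a goal decal under the cursor and pathfinds to it; manual movement cancels that command, stopping the character and removing the decal.
; Holding right mouse orbits the spring arm with clamped pitch, the wheel zooms it, and Left Shift sprints.
; Manual movement is relative to the spring arm's yaw.
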(event `self.ReceiveBeginPlay`
  (bind _ascharacter_shinbi (cast `/Game/RPG_Game/Blueprints/Character_shinbi` (`GameplayStatics.GetPlayerCharacter` 0)))
  (set `self.Shinbi` _ascharacter_shinbi))

(event `Key|LeftMouseButton`
  (params (Key :type "Key Structure"))
  (bind (_bblockinghit _binitialoverlap _time _distance _location) (`GameplayStatics.BreakHitResult` (`self.GetHitResultUnderCursorByChannel` "TraceTypeQuery1")))
  (:`Pressed`
    (`self.CancelMovementCommand`)
    (bind _returnvalue (`|SpawnActorFromClass` "/Game/RPG_Game/Actor/BP_GoalDecal.BP_GoalDecal_C" (`KismetMathLibrary.MakeTransform` _location) "Undefined" "OverrideRootScale" null self null))
    (set `self.CurrentGoalDecal` _returnvalue)
    (set `self.HasMouseMovementCommand?` true)
    (`AIBlueprintHelperLibrary.SimpleMoveToLocation` self _location)))

(event `Key|RightMouseButton`
  (params (Key :type "Key Structure"))
  (:`Pressed`
    (set `self.CanTurn?` true))
  (:`Released`
    (set `self.CanTurn?` false)))

(event `InputAxis|LookUp`
  (params (AxisValue :type "Float (single-precision)"))
  (bind _springarm (`/Game/RPG_Game/Blueprints/Character_shinbi.SpringArm` (`self.Shinbi`)))
  (bind (_returnvalue_location _returnvalue_rotation) (`KismetMathLibrary.BreakTransform` (`SceneComponent.GetRelativeTransform` _springarm)))
  ;[1 1 1] Character's Movement
  (if (and (`self.CanTurn?`) (!= AxisValue 0.0))
    (`SceneComponent.K2_SetRelativeRotation` _springarm (`KismetMathLibrary.MakeRotator` (.roll _returnvalue_rotation) (`KismetMathLibrary.FClamp` (+ (.pitch _returnvalue_rotation) AxisValue) -45.0 0.0) (.yaw _returnvalue_rotation)) false false)))

(event `InputAxis|Turn`
  (params (AxisValue :type "Float (single-precision)"))
  (bind _springarm (`/Game/RPG_Game/Blueprints/Character_shinbi.SpringArm` (`self.Shinbi`)))
  (bind (_returnvalue_location _returnvalue_rotation) (`KismetMathLibrary.BreakTransform` (`SceneComponent.GetRelativeTransform` _springarm)))
  ;[1 1 1] Character's Movement
  (if (and (`self.CanTurn?`) (!= AxisValue 0.0))
    (`SceneComponent.K2_SetRelativeRotation` _springarm (`KismetMathLibrary.MakeRotator` (.roll _returnvalue_rotation) (.pitch _returnvalue_rotation) (+ (.yaw _returnvalue_rotation) (* AxisValue 2.0))) false false)))

(event `InputAxis|MoveForward`
  (params (AxisValue :type "Float (single-precision)"))
  (bind (_returnvalue_location _returnvalue_rotation) (`KismetMathLibrary.BreakTransform` (`SceneComponent.GetRelativeTransform` (`/Game/RPG_Game/Blueprints/Character_shinbi.SpringArm` (`self.Shinbi`)))))
  ;[1 1 1] Character's Movement
  (if (!= AxisValue 0.0)
    (if (`self.HasMouseMovementCommand?`)
      (`self.CancelMovementCommand`))
    (`Pawn.AddMovementInput` (`self.Shinbi`) (`KismetMathLibrary.GetForwardVector` (`KismetMathLibrary.MakeRotator` 0.0 0.0 (.yaw _returnvalue_rotation))) AxisValue false)))

(event `InputAxis|MoveRight`
  (params (AxisValue :type "Float (single-precision)"))
  (bind (_returnvalue_location _returnvalue_rotation) (`KismetMathLibrary.BreakTransform` (`SceneComponent.GetRelativeTransform` (`/Game/RPG_Game/Blueprints/Character_shinbi.SpringArm` (`self.Shinbi`)))))
  ;[1 1 1] Character's Movement
  (if (!= AxisValue 0.0)
    (if (`self.HasMouseMovementCommand?`)
      (`self.CancelMovementCommand`))
    (`Pawn.AddMovementInput` (`self.Shinbi`) (`KismetMathLibrary.GetRightVector` (`KismetMathLibrary.MakeRotator` 0.0 0.0 (.yaw _returnvalue_rotation))) AxisValue false)))

(event `Key|MouseScrollUp`
  (params (Key :type "Key Structure"))
  (bind _springarm (`/Game/RPG_Game/Blueprints/Character_shinbi.SpringArm` (`self.Shinbi`)))
  ;[1 1 1] Character's Movement
  (:`Pressed`
    (set `SpringArmComponent.TargetArmLength` (`KismetMathLibrary.FClamp` (- (`SpringArmComponent.TargetArmLength` _springarm) (`self.SpringArmRate`)) 150.0 1500.0) _springarm)))

(event `Key|MouseScrollDown`
  (params (Key :type "Key Structure"))
  (bind _springarm (`/Game/RPG_Game/Blueprints/Character_shinbi.SpringArm` (`self.Shinbi`)))
  ;[1 1 1] Character's Movement
  (:`Pressed`
    (set `SpringArmComponent.TargetArmLength` (`KismetMathLibrary.FClamp` (+ (`SpringArmComponent.TargetArmLength` _springarm) (`self.SpringArmRate`)) 150.0 1500.0) _springarm)))

(event `Key|LeftShift`
  (params (Key :type "Key Structure"))
  (bind _charactermovement (`Character.CharacterMovement` (`self.Shinbi`)))
  ;[1 1 1] Character's Movement
  (:`Pressed`
    (set `CharacterMovementComponent.MaxWalkSpeed` 1500.0 _charactermovement))
  (:`Released`
    (set `CharacterMovementComponent.MaxWalkSpeed` 400.0 _charactermovement)))

(fn `CancelMovementCommand`
  (bind _currentgoaldecal (`self.CurrentGoalDecal`))
  (`/Engine/EditorBlueprintResources/StandardMacros.IsValid` _currentgoaldecal
    (:`Is Valid`
      (`MovementComponent.StopMovementImmediately` (`Character.CharacterMovement` (`self.Shinbi`)))
      (`self.K2_DestroyActor` _currentgoaldecal)
      (set `self.HasMouseMovementCommand?` false))
    (:`Is Not Valid`
      _))
  (return))

(fn `UserConstructionScript`)